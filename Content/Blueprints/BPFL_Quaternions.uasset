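; Blueprint function library of quaternion math helpers.
; QuatConjugate flips the sign of the vector part, while QuatNegate flips all four components.
; QuatToAxisAngle normalizes the vector part into an axis and derives the angle as twice the arccosine of W, without first normalizing the quaternion.
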(fn QuatConjugate
  (params (in :type Quat%20Structure))
  (bind (_x _y _z _w) (Utilities|Struct|BreakQuat in))
  (return (Utilities|Struct|MakeQuat (* _x -1.0) (* _y -1.0) (* _z -1.0) _w)))

(fn QuatNegate
  (params (in :type Quat%20Structure))
  (bind (_x _y _z _w) (Utilities|Struct|BreakQuat in))
  (return (Utilities|Struct|MakeQuat (* _x -1.0) (* _y -1.0) (* _z -1.0) (* _w -1.0))))

(fn QuattoAxisAngle
  (params (in :type Quat%20Structure))
  (bind (_x _y _z _w) (Utilities|Struct|BreakQuat in))
  (bind _output_get (LocalVariables|SetNorm (Math|Vector|MakeVector _x _y _z)))
  (bind _output_get_2 (LocalVariables|SetNorm (Math|Vector|Normalize _output_get)))
  (return _output_get_2 (* 2.0 (Math|Trig|Acos(Degrees) _w))))